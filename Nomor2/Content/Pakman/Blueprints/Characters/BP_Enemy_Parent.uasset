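; Parent Blueprint for Pac-Man-style enemies that either wander between random TargetPoints or hunt the player.
; A gated Tick drives AI moves and velocity-based eye visibility, opened by start and restart timers that retry until the player can gobble.
; Power pellets run a two-phase vulnerability timeline that forces wandering.
; Player overlap either awards escalating points and respawns this enemy at home, or kills the player and resets all enemies.
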(event `Power Pellet Eaten`
  ;[1 1 1] Vulenrability Sequence
  (set `self.bIsVulnerable?` true)
  (`self.Vulnerable`) ; Calls Event in Game Mode BP to alter the game's music
  (set `self.EnemyNavType` "NewEnumerator0")
  (`self.PickNewNavPoint`)
  (`Timeline|Vulnerability Sequence` :!via `PlayFromStart`
    (:`Finished`
      (`self.EnemyStateRegular`)
      (set `self.bIsVulnerable?` false)
      (if (`self.bIsHunterEnemy?`)
        (set `self.EnemyNavType` "NewEnumerator1")
        (`self.NoVulnerable`) ; Messages Game Mode BP top alter Muxic
        ;[1 1 1] Reset Enemy Point values
        (`self.ResetEnemyPointValues`)
        (else
          (set `self.EnemyNavType` "NewEnumerator0"))))
    (:`Start Phase #1`
      (`self.EnemyStateVulnerable01`))
    (:`Start Phase #2`
      (if (`self.bIsVulnerable?`)
        (`self.EnemyStateVulnerable02`)))))

(event `self.ReceiveBeginPlay`
  (`|ExecutionSequence`
    (:`then_0`
      ;[1 1 1] Reference to GameInstance
      (bind _asbp_game_instance (cast `/Game/Pakman/Blueprints/Framework/BP_GameInstance` (`GameplayStatics.GetGameInstance`)))
      (set `self.GameInstance` _asbp_game_instance)
      ;[1 1 1] Reference to all enemies
      (bind _outactors (`GameplayStatics.GetAllActorsOfClass` "BP_Enemy_Parent_C"))
      (set `self.Enemies` _outactors)
      ;[1 1 1] Reference to Player
      (bind _asbp_player (cast `/Game/Pakman/Blueprints/Characters/BP_Player` (`GameplayStatics.GetPlayerCharacter` 0)))
      (set `self.Player` _asbp_player)
      ;[1 1 1] Reference to Target Points
      (bind _outactors_2 (`GameplayStatics.GetAllActorsOfClass` "/Script/Engine.TargetPoint"))
      (set `self.TargetPoints` _outactors_2)
      ;[1 1 1] Stores enemy's spawn locale
      (set `self.EnemyRespawnLocation` (`self.K2_GetActorLocation`)))
    (:`then_1`
      ;[1 1 1] Opens gate for enemy nav
      (`self.SetEnemyStartTime`))))

(event `self.ReceiveTick`
  (params (DeltaSeconds :type "Float (single-precision)"))
  (`/Engine/EditorBlueprintResources/StandardMacros.Gate` true :!label _label
    (:`Exit`
      (`self.EyesMove`)
      (switch `/Game/Pakman/Blueprints/Framework/EnemyNavTypes` (`self.EnemyNavType`)
        (:`NewEnumerator0`
          (if (`self.bAssignedTargetPoint?`)
            ;[1 1 1] Enemy got to target point - pick new location
            (if (<= (`self.GetDistanceTo` (`self.EnemySelectedTarget`)) (`self.EnemyTargetAcceptanceRadius`))
              (`self.PickNewNavPoint`))
            (else
              ;[1 1 1] Wander Enemy Nav
              (`self.NavigationWander`))))
        (:`NewEnumerator1`
          ;[1 1 1] Hunter Enemy Nav
          (`self.NavigationHunter`))))))

(event `PickNewNavPoint`
  ;[1 1 1] Pick New Nav Point
  (`KismetSystemLibrary.Delay` 0.1)
  (set `self.bAssignedTargetPoint?` false)
  (goto _label :!via `Open`))

(event `SetEnemyStartTime`
  ;[1 1 1] Start Enemy Nav
  (`KismetSystemLibrary.K2_SetTimerDelegate` (delegate `StartNav`) (`self.EnemyStartTime`) :!label _label_2))

(event `self.Player_Collision.OnComponentBeginOverlap`
  (params (OverlappedComponent :type "PrimitiveComponent Object Reference") (OtherActor :type "Actor Object Reference") (OtherComp :type "PrimitiveComponent Object Reference") (OtherBodyIndex :type Integer) (bFromSweep :type Boolean) (SweepResult :type "HitResult Structure (by ref)"))
  (bind _returnvalue (`SceneComponent.K2_GetComponentToWorld` (`self.Pt_Spawn_Location`)))
  ;[1 1 1] Enemy Touched Player
  (bind _asbp_player (cast `/Game/Pakman/Blueprints/Characters/BP_Player` OtherActor))
  (`/Engine/EditorBlueprintResources/StandardMacros.IsValid` _asbp_player
    (:`Is Valid`
      (if (`self.bIsVulnerable?`)
        (`|ExecutionSequence`
          (:`then_0`
            ;[1 1 1] Pt Value Scores and FX
            (`self.EnemyEatenPoints`
              (:`1st Enemy Eaten`
                (`|SpawnActorFromClass` "/Game/Pakman/Blueprints/Misc/BP_Score_200.BP_Score_200_C" _returnvalue "Undefined" "OverrideRootScale" null null))
              (:`2nd Enemy Eaten`
                (`|SpawnActorFromClass` "/Game/Pakman/Blueprints/Misc/BP_Score_400.BP_Score_400_C" _returnvalue "Undefined" "OverrideRootScale" null null))
              (:`3rd Enemy Eaten`
                (`|SpawnActorFromClass` "/Game/Pakman/Blueprints/Misc/BP_Score_800.BP_Score_800_C" _returnvalue "Undefined" "OverrideRootScale" null null))
              (:`4th Enemy Eaten`
                (`|SpawnActorFromClass` "/Game/Pakman/Blueprints/Misc/BP_Score_1600.BP_Score_1600_C" _returnvalue "Undefined" "OverrideRootScale" null null))))
          (:`then_1`
            ;[1 1 1] Enemy Eaten - Respawn back at home
            (`self.CloseEnemyNavGate`) ; Stop just this enemy
            (`self.EnemyEatenFX`)
            (`PrimitiveComponent.SetCollisionResponseToChannel` (`self.Player_Collision`) "ECC_Pawn" "ECR_Ignore")
            (set `self.bIsVulnerable?` false)
            (`self.EnemyStateRegular` :!label _label_3)
            (`self.K2_SetActorLocation` (`self.EnemyRespawnLocation`))
            (`KismetSystemLibrary.Delay` 2.0)
            (`GameplayStatics.SpawnEmitterAtLocation` "/Game/Pakman/Particles/P_Monster_Death_Large.P_Monster_Death_Large" (`self.EnemyRespawnLocation`)) ; Respawn VFX
            (`PrimitiveComponent.SetCollisionResponseToChannel` (`self.Player_Collision`) "ECC_Pawn" "ECR_Overlap")
            (`KismetSystemLibrary.Delay` 1.0)
            (`self.SetActorHiddenInGame` false)
            (`self.SetEnemyRestartTime`)))
        (else
          ;[1 1 1] Send all enemies home
          (`self.KilledPlayer`)
          (`self.CloseEnemyNavGate` (`self.Enemies`)) ; Stop all enemies
          (`KismetSystemLibrary.Delay` 2.5)
          (`self.ResetEnemiesToHouse` (`self.Enemies`)))))))

(event `StartNav`
  ;[1 1 1] Start Enemy Nav
  (if (`/Game/Pakman/Blueprints/Characters/BP_Player.bShouldPlayerGobble?` (`self.Player`))
    (`ActorComponent.Activate` (`self.CharacterMovement`) false :!label _label_4)
    (set `self.bAssignedTargetPoint?` false)
    (goto _label :!via `Open`)
    (else
      (goto _label_2))))

(event `ResetEnemiesToHouse`
  ;[1 1 1] Enemy Eaten - Respawn back at home
  ;;[1 1 1] Reset to Enemy Spawn
  (`self.EnemySpawnOutFX`)
  (goto _label_3))

(event `CloseEnemyNavGate`
  ;[1 1 1] Stop Enemy Nav - player kill
  (`ActorComponent.Deactivate` (`self.CharacterMovement`))
  (goto _label :!via `Close`))

(event `SetEnemyRestartTime`
  ;[1 1 1] Restart Enemy Nav - After enemies sent home
  (`KismetSystemLibrary.K2_SetTimerDelegate` (delegate `RestartNav`) (`self.EnemyRestartTime`) :!label _label_5))

(event `RestartNav`
  ;[1 1 1] Restart Enemy Nav - After enemies sent home
  (if (`/Game/Pakman/Blueprints/Characters/BP_Player.bShouldPlayerGobble?` (`self.Player`))
    (goto _label_4)
    (else
      (goto _label_5))))

(fn `EnemyEatenFX`
  (`GameplayStatics.SpawnEmitterAtLocation` "/Game/Pakman/Particles/P_Death.P_Death" (`SceneComponent.K2_GetComponentLocation` (`self.CapsuleComponent`)))
  (`GameplayStatics.PlaySound2D` "/Game/Pakman/Audio/SFX-EatEnemy_Cue.SFX-EatEnemy_Cue" 1.0 1.0 0.0 null null)
  (`self.SetActorHiddenInGame` true))

(fn `EnemySpawnOutFX`
  (`GameplayStatics.SpawnEmitterAtLocation` "/Game/Pakman/Particles/P_SpawnOut_Enemy.P_SpawnOut_Enemy" (`SceneComponent.K2_GetComponentLocation` (`self.CapsuleComponent`))) ; Spawn Out VFX
  (`self.SetActorHiddenInGame` true))

(fn `EnemyStateRegular`
  (`SceneComponent.SetVisibility` (`self.Enemy_Vulnerable_01`) false false)
  (`SceneComponent.SetVisibility` (`self.Enemy_Vulnerable_02`) false false)
  (`self.EyesLookDown`))

(fn `EnemyStateVulnerable01`
  (`SceneComponent.SetVisibility` (`self.Enemy_Vulnerable_02`) false false)
  (`SceneComponent.SetVisibility` (`self.Enemy_Down`) false false)
  (`SceneComponent.SetVisibility` (`self.Enemy_Vulnerable_01`) true false))

(fn `EnemyStateVulnerable02`
  (`SceneComponent.SetVisibility` (`self.Enemy_Down`) false false)
  (`SceneComponent.SetVisibility` (`self.Enemy_Vulnerable_01`) false false)
  (`SceneComponent.SetVisibility` (`self.Enemy_Vulnerable_02`) true false))

(fn `EyesLookDown`
  (`SceneComponent.SetVisibility` (`self.Enemy_Down`) true false)
  (`SceneComponent.SetVisibility` (`self.Enemy_Up`) false false)
  (`SceneComponent.SetVisibility` (`self.Enemy_Right`) false false)
  (`SceneComponent.SetVisibility` (`self.Enemy_Left`) false false))

(fn `EyesLookLeft`
  (`SceneComponent.SetVisibility` (`self.Enemy_Left`) true false)
  (`SceneComponent.SetVisibility` (`self.Enemy_Up`) false false)
  (`SceneComponent.SetVisibility` (`self.Enemy_Down`) false false)
  (`SceneComponent.SetVisibility` (`self.Enemy_Right`) false false))

(fn `EyesLookRight`
  (`SceneComponent.SetVisibility` (`self.Enemy_Right`) true false)
  (`SceneComponent.SetVisibility` (`self.Enemy_Up`) false false)
  (`SceneComponent.SetVisibility` (`self.Enemy_Left`) false false)
  (`SceneComponent.SetVisibility` (`self.Enemy_Down`) false false))

(fn `EyesLookUp`
  (`SceneComponent.SetVisibility` (`self.Enemy_Up`) true false)
  (`SceneComponent.SetVisibility` (`self.Enemy_Right`) false false)
  (`SceneComponent.SetVisibility` (`self.Enemy_Left`) false false)
  (`SceneComponent.SetVisibility` (`self.Enemy_Down`) false false))

(fn `EyesMove`
  (bind (_velocity_x _velocity_y) (`KismetMathLibrary.BreakVector` (`MovementComponent.Velocity` (`self.CharacterMovement`))))
  (bind _velocity_x_2 (`KismetMathLibrary.BreakVector` (`MovementComponent.Velocity` (`self.CharacterMovement`))))
  (bind (_velocity_x_3 _velocity_y_2) (`KismetMathLibrary.BreakVector` (`MovementComponent.Velocity` (`self.CharacterMovement`))))
  (if (`self.bIsVulnerable?`)
    (`self.EyesNone`)
    (elif (>= (`KismetMathLibrary.Abs` _velocity_x) (`KismetMathLibrary.Abs` _velocity_y))
      (if (>= _velocity_x_2 0.0)
        (`self.EyesLookRight`)
        (else
          (`self.EyesLookLeft`)))
      (elif (>= _velocity_y_2 0.0)
        (`self.EyesLookDown`)
        (else
          (`self.EyesLookUp`))))))

(fn `EyesNone`
  (`SceneComponent.SetVisibility` (`self.Enemy_Right`) false false)
  (`SceneComponent.SetVisibility` (`self.Enemy_Left`) false false)
  (`SceneComponent.SetVisibility` (`self.Enemy_Down`) false false)
  (`SceneComponent.SetVisibility` (`self.Enemy_Up`) false false))

(fn `NavigationHunter`
  (`AIController.MoveToLocation` (`AIBlueprintHelperLibrary.GetAIController` (`self.GetController`)) (`SceneComponent.K2_GetComponentLocation` (`Character.CapsuleComponent` (`self.Player`))) -1.0 true true false true null true))

(fn `NavigationWander`
  (bind _targetpoints (`self.TargetPoints`))
  (bind _output_get (set `self.EnemySelectedTarget` (`|GetArrayItem` _targetpoints (`KismetMathLibrary.RandomInteger` (`KismetArrayLibrary.Array_Length` _targetpoints)))))
  (`AIController.MoveToLocation` (`AIBlueprintHelperLibrary.GetAIController` (`self.GetController`)) (`self.K2_GetActorLocation` _output_get) -1.0 true true false true null true)
  (set `self.bAssignedTargetPoint?` true))

(fn `ResetEnemyPointValues`
  (bind _player (`self.Player`))
  (set `/Game/Pakman/Blueprints/Characters/BP_Player.bHaveEatenOneEnemy?` false _player)
  (set `/Game/Pakman/Blueprints/Characters/BP_Player.bHaveEatenTwoEnemies?` false _player)
  (set `/Game/Pakman/Blueprints/Characters/BP_Player.bHaveEatenThreeEnemies?` false _player)
  (set `/Game/Pakman/Blueprints/Characters/BP_Player.bHaveEatenFourEnemies?` false _player))

(fn `UserConstructionScript`)