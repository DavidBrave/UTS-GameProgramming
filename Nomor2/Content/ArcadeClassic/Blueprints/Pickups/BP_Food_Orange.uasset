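; BP_Food_Orange is an orange bonus fruit pickup for an arcade game, announcing its spawn with a scaled-up particle burst and sound.
; When BP_Player overlaps its collision, it plays eaten effects, removes its collision and visual components, spawns a BP_Score_1000 actor, and destroys itself after a delay.
; The same overlap adds OrangePoints through BP_GameInstance and runs its 1-up check.
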(event `self.ReceiveBeginPlay`
  ;[1 1 1] Goodie Spawn FX
  (`self.Spawn FX`))

(event `self.Collision.OnComponentBeginOverlap`
  (params (OverlappedComponent :type "PrimitiveComponent Object Reference") (OtherActor :type "Actor Object Reference") (OtherComp :type "PrimitiveComponent Object Reference") (OtherBodyIndex :type Integer) (bFromSweep :type Boolean) (SweepResult :type "HitResult Structure (by ref)"))
  (cast `/Game/ArcadeClassic/Blueprints/Characters/BP_Player` OtherActor)
  (`|ExecutionSequence`
    (:`then_0`
      ;[1 1 1] Fruit Eaten Handling
      (`GameplayStatics.PlaySound2D` "/Game/ArcadeClassic/Audio/SFX-EatSpecial_Cue.SFX-EatSpecial_Cue" 1.0 1.0 0.0 null null)
      (`ActorComponent.Activate` (`self.VFX_Eaten`) false)
      (`ActorComponent.K2_DestroyComponent` (`self.Collision`))
      (`ActorComponent.K2_DestroyComponent` (`self.SM_Orange`))
      (`ActorComponent.K2_DestroyComponent` (`self.SM_Leaf`))
      (`ActorComponent.K2_DestroyComponent` (`self.VFX_Glow`))
      (`ActorComponent.K2_DestroyComponent` (`self.RotatingMovement`))
      (`|SpawnActorFromClass` "/Game/ArcadeClassic/Blueprints/Misc/BP_Score_1000.BP_Score_1000_C" (`KismetMathLibrary.MakeTransform` (`SceneComponent.K2_GetComponentLocation` (`self.DefaultSceneRoot`))) "Undefined" "OverrideRootScale" null null)
      (`KismetSystemLibrary.Delay` 5.0)
      (`self.K2_DestroyActor`))
    (:`then_1`
      ;[1 1 1] Increment Score
      (bind _asbp_game_instance (cast `/Game/ArcadeClassic/Blueprints/Framework/BP_GameInstance` (`GameplayStatics.GetGameInstance`)))
      (`/Game/ArcadeClassic/Blueprints/Framework/BP_GameInstance.AddPoints` _asbp_game_instance (`self.OrangePoints`))
      (`/Game/ArcadeClassic/Blueprints/Framework/BP_GameInstance.1up Check` _asbp_game_instance))))

(fn `Spawn FX`
  (bind _returnvalue (`GameplayStatics.SpawnEmitterAtLocation` "/Game/ArcadeClassic/Particles/P_levelUp.P_levelUp" (`SceneComponent.K2_GetComponentLocation` (`self.Collision`))))
  (`SceneComponent.SetWorldScale3D` _returnvalue (3.0 3.0 3.0))
  (`GameplayStatics.PlaySound2D` "/Game/ArcadeClassic/Audio/SFX-FruitSpawn_Cue.SFX-FruitSpawn_Cue" 1.0 1.0 0.0 null null))

(fn `UserConstructionScript`)